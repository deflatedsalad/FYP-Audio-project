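; BP_Node is an audio node actor that plays an attached, attenuated sound and traces lines to other nodes and a listener.
; BeginPlay registers its audio bus to the master submix and spawns the sound, while StartBus toggles the bus.
; GetOtherNodes stores the listener and the node list minus itself for CastRayToNodes, whose Visibility traces draw debug lines but leave results unused.
; Neither function is called within this Blueprint.
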(event EventBeginPlay
  (Class|AudioMixerBlueprintLibrary|RegisterAudioBustoSubmix "/Engine/EngineSounds/Submixes/MasterSubmixDefault.MasterSubmixDefault" (Variables|Default|Getbus))
  (Audio|SpawnSoundAttached (Variables|Default|GetSource) (Variables|Default|GetAudio) "None" "0, 0, 0" "0, 0, 0" "KeepRelativeOffset" false 1.0 1.0 0.0 "/Game/SA_Attenuation.SA_Attenuation" 0 false))

(event Collision|EventActorBeginOverlap
  (params (OtherActor :type Actor%20Object%20Reference)))

(event EventTick
  (params (DeltaSeconds :type Float%20%28single-precision%29)))

(event EventStartBus
  (params (Enable :type Boolean))
  (bind _bus (Variables|Default|Getbus))
  (if Enable
    (Class|AudioMixerBlueprintLibrary|StartAudioBus _bus)
    (Development|PrintString "enabled")
    (else
      (Class|AudioMixerBlueprintLibrary|StopAudioBus _bus)
      (Development|PrintString "disabled"))))

(fn ConstructionScript)

(fn GetOtherNodes
  (params (nodes :type Array%20of%20BP%20Node%20Object%20References) (CurrentIndex :type Integer) (Listener :type Actor%20Object%20Reference))
  (bind _output_get (Variables|Default|SetNodes nodes))
  (Utilities|Array|RemoveIndex _output_get CurrentIndex)
  (Variables|Default|SetListener Listener))

(fn CastRaytoNodes
  (bind _mesh (Variables|Default|GetMesh))
  (bind _returnvalue (Transformation|GetWorldLocation _mesh))
  (for _array_element (Variables|Default|GetNodes)
    (Collision|LineTraceByChannel _returnvalue (Transformation|GetWorldLocation (Variables|BP_Node_C|GetMesh _array_element)) "TraceTypeQuery1" false 0 "ForDuration")
    (Collision|LineTraceByChannel _returnvalue (Transformation|GetActorLocation (Variables|Default|GetListener)) "TraceTypeQuery1" false 0 "ForDuration")))