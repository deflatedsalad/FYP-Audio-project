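; BP_character is a player character with first-person style walk and look controls driven by Enhanced Input.
; BeginPlay adds the default mapping context if missing, and walk input feeds CharacterMovement a speed-scaled vector rotated by the full camera rotation.
; Look input sets the camera's relative rotation from its world rotation plus input, with pitch clamped.
; A Z debug key tells BPNodeManager to cast rays.
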(event Input|EnhancedActionEvents|EnhancedInputActionIA_WAlk
  (params (ActionValue :type Vector%202D%20Structure) (ElapsedSeconds :type Float%20%28double-precision%29) (TriggeredSeconds :type Float%20%28double-precision%29) (InputAction :type Input%20Action%20Object%20Reference :default "/Game/PlayerControls/Inputs/IA_WAlk.IA_WAlk"))
  (Class|PawnMovementComponent|AddInputVector (Variables|Character|GetCharacterMovement) (Math|Vector|RotateVector (Math|Conversions|ToVector(Vector2D) (* ActionValue (Variables|Default|Getspeed))) (Transformation|GetWorldRotation (Variables|Default|GetCamera))) false))

(event Input|EnhancedActionEvents|EnhancedInputActionIA_look
  (params (ActionValue :type Vector%202D%20Structure) (ElapsedSeconds :type Float%20%28double-precision%29) (TriggeredSeconds :type Float%20%28double-precision%29) (InputAction :type Input%20Action%20Object%20Reference :default "/Game/PlayerControls/Inputs/IA_look.IA_look"))
  (bind _camera (Variables|Default|GetCamera))
  (bind _returnvalue (Transformation|GetWorldRotation _camera))
  (Transformation|SetRelativeRotation (Variables|Default|GetCamera) (Math|Rotator|MakeRotator (.roll _returnvalue) (Math|Float|Clamp(Float) (+ (.y ActionValue) (.pitch _returnvalue)) -6e+01 6e+01) (+ (.x ActionValue) (.yaw _returnvalue))) false false))

(event EventBeginPlay
  (bind _returnvalue (Game|GetPlayerController 0))
  (bind _returnvalue_2 (PlayerController|LocalPlayerSubsystems|GetEnhancedInputLocalPlayerSubsystem _returnvalue))
  (if (not (.ReturnValue (Class|EnhancedInputSubsystemInterface|HasMappingContext _returnvalue_2 "/Game/PlayerControls/Inputs/IMC_default.IMC_default")))
    (Input|AddMappingContext _returnvalue_2 "/Game/PlayerControls/Inputs/IMC_default.IMC_default" 0 "(bIgnoreAllPressedKeysUntilRelease=True,bForceImmediately=False,bNotifyUserSettings=False)")))

(event Collision|EventActorBeginOverlap
  (params (OtherActor :type Actor%20Object%20Reference)))

(event EventTick
  (params (DeltaSeconds :type Float%20%28single-precision%29)))

(event Input|KeyboardEvents|DebugKeyZ
  (params (Key :type Key%20Structure :default "None") (ActionValue :type Input%20Action%20Value%20Structure))
  (:Pressed
    (Default|CastRays (Variables|Default|GetBP_nodeManager))))

(fn ConstructionScript)