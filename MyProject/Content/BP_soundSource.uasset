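; Sound source Blueprint that plays a wave through a MetaSound, simulating propagation delay and obstruction to acoustic nodes.
; Initialise stores the audio component and every BP_Node, then passes in the wave asset.
; PlaySound line-traces from its owner to each node, switching that node's bus on only if the trace hits a node.
; For clear paths, distance over speed of sound sets an indexed MetaSound delay parameter before playback.
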(event EventBeginPlay
  (Actor|GetActorOfClass 0)
  (bind _asbp_character (Utilities|Casting|CastToBP_character (Game|Player|GetPlayerPawn 0)))
  (Variables|Default|SetNodeManager (Components|GetChildComponent (Variables|/Game/PlayerControls/BP_character.BP_character_C|GetBP_nodeManager _asbp_character) 0)))

(fn Initialise
  (params (AudioComponent :type Audio%20Component%20Object%20Reference) (inputWaveFile :type Sound%20Wave%20Object%20Reference))
  (Variables|Default|SetAudio%20Component AudioComponent)
  (bind _outactors (Actor|GetAllActorsOfClass "/Game/BP_Node.BP_Node_C"))
  (Variables|Default|SetNodes _outactors)
  (Class|AudioComponent|SetWaveParameter (Variables|Default|GetAudio%20Component) "Wave Asset" inputWaveFile))

(fn PlaySound
  (for (_array_element _array_index) (Variables|Default|GetNodes)
    ;[1 1 1] line trace between the sound source and the nodes to get the distance and if they are obstructed
    (Variables|Default|SetArray%20Index _array_index)
    (Variables|Default|SetArray%20Element _array_element)
    (bind _outhit (Collision|LineTraceByChannel (Transformation|GetActorLocation (Components|GetOwner)) (Transformation|GetWorldLocation (Variables|/Game/BP_Node.BP_Node_C|GetMesh _array_element)) "TraceTypeQuery1" false 0 "None"))
    ;[1 1 1] determine if audio buses should be active based on if there was anything between the nodes and the source
    (if (== (Utilities|GetClass (.HitActor (Collision|BreakHitResult _outhit))) "/Game/BP_Node.BP_Node_C")
      (Class|BIStartBus|StartBus(Message) (Variables|Default|GetArray%20Element) true)
      ;[1 1 1] set delay time for the connection to each node based on distance
      (Audio|Parameter|SetFloatParameter (Variables|Default|GetAudio%20Component) (Utilities|String|StringToName (Utilities|String|Append "Delay Time " (Utilities|String|ToString(Integer) (Variables|Default|GetArray%20Index)))) (/ (/ (.Distance (Collision|BreakHitResult _outhit)) 1e+02) (Variables|Default|GetSpeedOfSound)) :!class /Script/AudioExtensions.AudioParameterControllerInterface)
      (else
        (Class|BIStartBus|StartBus(Message) (Variables|Default|GetArray%20Element) false))))
  ;[1 1 1] trigger the starting metasound to play the sound file
  (Audio|Components|Audio|Play (Variables|Default|GetAudio%20Component) 0.0))