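; Manager Blueprint that sets up and coordinates all BP_Node actors in the level.
; On BeginPlay it gathers every node and passes each the full list, its own index and player character 0 as the listener.
; It then has every node cast rays to the other nodes.
; An UpdatePlayerPosition event relays a given player position to all nodes.
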(event Custom|CastRays
  ;[1 1 1] cast a ray between each node
  (for _array_element (Variables|Default|GetNodes)
    (Default|CastRaytoNodes _array_element)))

(event Custom|UpdatePlayerPosition
  (params (playerPosition :type Vector))
  (for _array_element (Variables|Default|GetNodes)
    (Default|UpdatePlayerLocation _array_element playerPosition)))

(event EventBeginPlay
  ;[1 1 1] give each node an array containing all existing nodes
  (bind _outactors (Actor|GetAllActorsOfClass "/Game/BP_Node.BP_Node_C"))
  (bind _output_get (Variables|Default|SetNodes _outactors))
  (for (_array_element _array_index) _output_get
    (Default|GetOtherNodes _array_element _output_get _array_index (Game|GetPlayerCharacter 0)))
  (CallFunction|CastRays))